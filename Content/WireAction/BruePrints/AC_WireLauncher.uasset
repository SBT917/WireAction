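; AC_WireLauncher is an actor component that fires and removes a cable wire for its owning Character.
; WireDirectionTrace line-traces along a direction on the Visibility channel and returns hit success and location.
; WireLaunch spawns a BP_Wire snapped to a given component socket and a BP_WireTarget at the target, linking the cable's end to it and passing both references to the wire.
; DestroyWire destroys both actors.
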(event `self.ReceiveBeginPlay`
  (bind _ascharacter (cast `Character` (`self.GetOwner`)))
  (set `self.OwnerCharacter` _ascharacter))

(event `self.ReceiveTick`
  (params (DeltaSeconds :type "Float (single-precision)")))

(fn `DestroyWire`
  (bind _wire (`self.Wire`))
  (bind _wiretarget (`self.WireTarget`))
  (if (`KismetSystemLibrary.IsValid` _wire)
    (`Actor.K2_DestroyActor` _wire)
    (if (`KismetSystemLibrary.IsValid` _wiretarget)
      (`Actor.K2_DestroyActor` _wiretarget))))

(fn `Wire Launch`
  (params (TargetPosition :type "Vector Structure") (AttachComponent :type "SceneComponent Object Reference") (SocketName :type Name))
  (bind _wire (`self.Wire`))
  (bind _returnvalue (`|SpawnActorFromClass` "/Game/WireAction/BruePrints/BP_Wire.BP_Wire_C" (`KismetMathLibrary.MakeTransform` (`Actor.K2_GetActorLocation` (`self.GetOwner`))) "AlwaysSpawn" "MultiplyWithRoot" null null))
  (`Actor.K2_AttachToComponent` _returnvalue AttachComponent SocketName "SnapToTarget" "SnapToTarget" "SnapToTarget" true)
  (bind _output_get (set `self.Wire` _returnvalue))
  (bind _returnvalue_2 (`|SpawnActorFromClass` "/Game/WireAction/BruePrints/BP_WireTarget.BP_WireTarget_C" (`KismetMathLibrary.MakeTransform` TargetPosition) "Undefined" "MultiplyWithRoot" null null))
  (bind _output_get_2 (set `self.WireTarget` _returnvalue_2))
  (`CableComponent.SetAttachEndTo` (`CableActor.CableComponent` _output_get) _output_get_2 "DefaultSceneRoot" "None")
  (set `/Game/WireAction/BruePrints/BP_Wire.OwnerCharacter` (`self.OwnerCharacter`) _wire)
  (set `/Game/WireAction/BruePrints/BP_Wire.WireTarget` _output_get_2 _wire))

(fn `WireDirectionTrace`
  (params (StartPos :type "Vector Structure") (Direction :type "Vector Structure"))
  (returns (IsSucces :type Boolean) (Position :type "Vector Structure"))
  (bind (_outhit _returnvalue) (`KismetSystemLibrary.LineTraceSingle` :`Start` StartPos :`End` (+ StartPos (* Direction (`self.TraceLength`))) :`TraceChannel` "TraceTypeQuery1" :`DrawDebugType` "ForDuration"))
  (return _returnvalue (`.Location` (`GameplayStatics.BreakHitResult` _outhit))))